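; Pinball slingshot bumper that awards score and kicks the ball away when a BP_Ball overlaps it.
; The overlap adds SlingScore through PinballGamemode, pushes the ball along the capsule's forward vector by SlingForce and plays a sound.
; The SlingBounce timeline animates the bounce through a scalar parameter on a dynamic material instance, created in the construction script for one mesh slot.
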(event EventBeginPlay)

(event Collision|EventActorBeginOverlap
  (params (OtherActor :type Actor%20Object%20Reference))
  (bind _asbp_ball (Utilities|Casting|CastToBP_Ball OtherActor))
  (bind _aspinball_gamemode (Utilities|Casting|CastToPinballGamemode (Game|GetGameMode))
    (:then
      (Default|AddScore _aspinball_gamemode (Variables|Default|GetSlingScore)))
    (:CastFailed
      _))
  (Physics|AddImpulse (Variables|/Game/PinballGame/Blueprints/BP_Ball.BP_Ball_C|GetBall _asbp_ball) (* (Math|Vector|GetForwardVector (Variables|Default|GetCapsule)) (Variables|Default|GetSlingForce)) "None" false)
  (Audio|Components|Audio|Play (Variables|Default|GetAudio) 0.0)
  (bind _bouncealpha (Timeline|SlingBounce PlayFromStart)
    (:Update
      (bind _asmaterial_instance_dynamic (Utilities|Casting|CastToMaterialInstanceDynamic (Rendering|Material|GetMaterial (Variables|Default|GetSlingShotMesh) 2)))
      (Rendering|Material|SetScalarParameterValue _asmaterial_instance_dynamic "PerecentOut" _bouncealpha :!class /Script/Engine.MaterialInstanceDynamic))))

(event EventTick
  (params (DeltaSeconds :type Float%20%28single-precision%29)))

(fn ConstructionScript
  (Rendering|Material|CreateDynamicMaterialInstance (Variables|Default|GetSlingShotMesh) 2 0 :!class /Script/Engine.PrimitiveComponent))
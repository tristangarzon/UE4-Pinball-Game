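; BP_Flipper is a pinball flipper actor configured as left or right through FlipType.
; The construction script picks mirrored start and end yaw rotations and the matching sound, mirroring the mesh on X for the right side.
; Flip rotates the flipper to its end rotation over FlipTime and plays the sound, while Flop rotates it back to the start.
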(event Custom|Flip
  (Components|MoveComponentTo (Variables|Default|GetFlipper) "0, 0, 0" (Variables|Default|GetEndRotation) false false (Variables|Default|GetFlipTime) false)
  (Audio|Components|Audio|Play (Variables|Default|GetFlipperAudio) 0.0))

(event Custom|Flop
  (Components|MoveComponentTo (Variables|Default|GetFlipper) "0, 0, 0" (Variables|Default|GetStartRotation) false false (Variables|Default|GetFlipTime) false))

(event EventBeginPlay)

(event Collision|EventActorBeginOverlap
  (params (OtherActor :type Actor%20Object%20Reference)))

(event EventTick
  (params (DeltaSeconds :type Float%20%28single-precision%29)))

(fn ConstructionScript
  (Variables|Default|SetStartRotation (Utilities|Select :Index (Variables|Default|GetFlipType) :NewEnumerator0 "0,20.000000, 0" :NewEnumerator1 "0.000000,-20.000000,0.000000"))
  (Variables|Default|SetEndRotation (Utilities|Select :Index (Variables|Default|GetFlipType) :NewEnumerator0 "0,-20.000000, 0" :NewEnumerator1 "0.000000,20.000000,0.000000"))
  (Transformation|SetRelativeRotation (Variables|Default|GetFlipper) (Variables|Default|GetStartRotation) false false)
  (switch Utilities|FlowControl|Switch|SwitchonFlipType (Variables|Default|GetFlipType)
    (:NewEnumerator0
      (Audio|Components|Audio|SetSound (Variables|Default|GetFlipperAudio) "/Game/PinballGame/Assets/Sounds/Pinball_FlipperLeft.Pinball_FlipperLeft"))
    (:NewEnumerator1
      (Transformation|SetRelativeScale3D (Variables|Default|GetFlipper) "-1.000000,1.000000,1.000000")
      (Audio|Components|Audio|SetSound (Variables|Default|GetFlipperAudio) "/Game/PinballGame/Assets/Sounds/Pinball_FlipperRight.Pinball_FlipperRight"))))
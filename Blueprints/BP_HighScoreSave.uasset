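; BP_HighScoreSave stores a high score table, presumably as save data, capped at MaxHighScore entries.
; AddHighScore appends a new entry, sorts the table and trims it to the cap.
; SortSaveData selection-sorts descending by repeatedly moving the CheckHighestScore result into TempSaveStruct.
; CheckLowestScore is unused here and uses the same greater-than test, so it actually returns the highest score.
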(fn CheckLowestScore
  (for (_array_element _array_index) (Variables|Default|GetSaveStruct)
    (if (== _array_index 0)
      (LocalVariables|SetLowestScore (.score _array_element))
      (LocalVariables|SetLowestIndex _array_index)
      (elif (> (.score _array_element) (LocalVariables|GetLowestScore))
        (LocalVariables|SetLowestScore (.score _array_element))
        (LocalVariables|SetLowestIndex _array_index))))
  (return (Utilities|Array|Get(acopy) (Variables|Default|GetSaveStruct) (LocalVariables|GetLowestIndex)) (LocalVariables|GetLowestIndex)))

(fn CheckHighestScore
  (for (_array_element _array_index) (Variables|Default|GetSaveStruct)
    (if (== _array_index 0)
      (LocalVariables|SetHighestScore (.score _array_element))
      (LocalVariables|SetHighestIndex _array_index)
      (elif (> (.score _array_element) (LocalVariables|GetHighestScore))
        (LocalVariables|SetHighestScore (.score _array_element))
        (LocalVariables|SetHighestIndex _array_index))))
  (return (Utilities|Array|Get(acopy) (Variables|Default|GetSaveStruct) (LocalVariables|GetHighestIndex)) (LocalVariables|GetHighestIndex)))

(fn SortSaveData
  (while (> (Utilities|Array|Length (Variables|Default|GetSaveStruct)) 0)
    (bind (_highestscorestruct _highestscoreindex) (CallFunction|CheckHighestScore))
    (Utilities|Array|Add (LocalVariables|GetTempSaveStruct) _highestscorestruct)
    (Utilities|Array|RemoveIndex (Variables|Default|GetSaveStruct) _highestscoreindex))
  (Variables|Default|SetSaveStruct (LocalVariables|GetTempSaveStruct)))

(fn AddHighScore
  (params (NewScore :type BP%20Highscore%20Struct%20Structure))
  (bind _savestruct (Variables|Default|GetSaveStruct))
  (Utilities|Array|Add (Variables|Default|GetSaveStruct) NewScore)
  (CallFunction|SortSaveData)
  (Utilities|Array|Resize _savestruct (Math|Integer|Min(Integer) (Variables|Default|GetMaxHighScore) (Utilities|Array|Length _savestruct))))